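; BP_hack_computer is an interactable computer that the player hacks by repeatedly pressing E while inside its Box trigger.
; Overlap shows or hides the controller's HackWidget and syncs it to this computer's hacked state.
; Each press in range increments the widget's Timeheld until MaxTimeHeld marks the computer hacked.
; Progress lives on the shared widget and is never reset here, despite the hold-style naming.
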(event OnComponentBeginOverlap(Box)
  (params (OverlappedComponent :type Primitive%20Component%20Object%20Reference) (OtherActor :type Actor%20Object%20Reference) (OtherComp :type Primitive%20Component%20Object%20Reference) (OtherBodyIndex :type Integer) (bFromSweep :type Boolean) (SweepResult :type Hit%20Result%20Structure%20%28by%20ref%29))
  (Utilities|Casting|CastToFirstPersonCharacter OtherActor)
  (bind _asbp_custom_player_controller (Utilities|Casting|CastToBP_CustomPlayerController (Game|GetPlayerController 0)))
  (Default|ShowCanvas (Variables|/Game/Wout/Hud/BP_CustomPlayerController.BP_CustomPlayerController_C|GetHackWidget _asbp_custom_player_controller))
  (Default|SettoHacked (Variables|/Game/Wout/Hud/BP_CustomPlayerController.BP_CustomPlayerController_C|GetHackWidget _asbp_custom_player_controller) (Variables|Default|GetHackedB))
  (Variables|Default|SetIsInRange true))

(event OnComponentEndOverlap(Box)
  (params (OverlappedComponent :type Primitive%20Component%20Object%20Reference) (OtherActor :type Actor%20Object%20Reference) (OtherComp :type Primitive%20Component%20Object%20Reference) (OtherBodyIndex :type Integer))
  (Utilities|Casting|CastToFirstPersonCharacter OtherActor)
  (bind _asbp_custom_player_controller (Utilities|Casting|CastToBP_CustomPlayerController (Game|GetPlayerController 0)))
  (Default|HideCanvas (Variables|/Game/Wout/Hud/BP_CustomPlayerController.BP_CustomPlayerController_C|GetHackWidget _asbp_custom_player_controller))
  (Variables|Default|SetIsInRange false))

(event Custom|Press%20hack
  (if (Variables|Default|GetIsInRange)
    (if (not (Variables|Default|GetHackedB))
      (bind _asbp_custom_player_controller (Utilities|Casting|CastToBP_CustomPlayerController (Game|GetPlayerController 0)))
      (Utilities|FlowControl|Sequence
        (:then_0
          (Variables|/Game/Wout/bluePrints/P_holdE.P_holdE_C|Settimeheld (Variables|/Game/Wout/Hud/BP_CustomPlayerController.BP_CustomPlayerController_C|GetHackWidget _asbp_custom_player_controller) (+ (Variables|/Game/Wout/bluePrints/P_holdE.P_holdE_C|Gettimeheld (Variables|/Game/Wout/Hud/BP_CustomPlayerController.BP_CustomPlayerController_C|GetHackWidget _asbp_custom_player_controller)) 0.2)))
        (:then_1
          (if (>= (Variables|/Game/Wout/bluePrints/P_holdE.P_holdE_C|Gettimeheld (Variables|/Game/Wout/Hud/BP_CustomPlayerController.BP_CustomPlayerController_C|GetHackWidget _asbp_custom_player_controller)) (Variables|/Game/Wout/bluePrints/P_holdE.P_holdE_C|GetMaxTimeHeld (Variables|/Game/Wout/Hud/BP_CustomPlayerController.BP_CustomPlayerController_C|GetHackWidget _asbp_custom_player_controller)))
            (CallFunction|SetHacked true)
            (Default|SettoHacked (Variables|/Game/Wout/Hud/BP_CustomPlayerController.BP_CustomPlayerController_C|GetHackWidget _asbp_custom_player_controller) true)))))))

(event EventBeginPlay
  (bind _returnvalue (Game|GetPlayerController 0))
  (Input|EnableInput _returnvalue)
  (Utilities|Casting|CastToBP_CustomPlayerController _returnvalue))

(event Input|KeyboardEvents|E
  (params (Key :type Key%20Structure :default "None"))
  (:Pressed
    (CallFunction|PressHack)))

(fn ConstructionScript)

(fn SetHacked
  (params (isHacked :type Boolean))
  (bind _output_get (Variables|Default|SetHackedB isHacked))
  (Development|PrintString (Utilities|String|Append (LocalVariables|GetNewLocalVar) (Utilities|String|ToString(Boolean) _output_get))))