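; Spline-driven actor that builds a continuous deformed mesh along an editable spline.
; The construction script adds one spline mesh component per segment between consecutive points, all using the Mesh variable and attached to the scene root.
; Each segment takes its start and end positions and tangents from the spline in local space.
; Per-point spline scale, converted to 2D, sets each segment's start and end scale, letting the cross-section vary along the path.
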(fn ConstructionScript
  (bind _spline (Variables|Default|GetSpline))
  (bind _spline_2 (Variables|Default|GetSpline))
  (for _index (range 0 (- (Spline|GetNumberOfSplinePoints (Variables|Default|GetSpline)) 2))
    (bind _returnvalue (AddComponent|AddSplineMeshComponent false))
    (Components|StaticMesh|SetStaticMesh _returnvalue (Variables|Default|GetMesh))
    (Transformation|AttachComponentToComponent _returnvalue (Variables|Default|GetDefaultSceneRoot) "None" "KeepRelative" "KeepRelative" "KeepRelative" true)
    (SplineMesh|SetStartandEnd _returnvalue (.Location (Spline|GetLocationandTangentatSplinePoint _spline _index "Local")) (.Tangent (Spline|GetLocationandTangentatSplinePoint _spline _index "Local")) (.Location (Spline|GetLocationandTangentatSplinePoint _spline (+ _index 1) "Local")) (.Tangent (Spline|GetLocationandTangentatSplinePoint _spline (+ _index 1) "Local")) true :!class /Script/Engine.SplineMeshComponent)
    (SplineMesh|SetStartScale _returnvalue (Math|Conversions|ToVector2D(Vector) (Spline|GetScaleatSplinePoint _spline_2 _index)) true :!class /Script/Engine.SplineMeshComponent)
    (SplineMesh|SetEndScale _returnvalue (Math|Conversions|ToVector2D(Vector) (Spline|GetScaleatSplinePoint _spline_2 (+ _index 1))) true :!class /Script/Engine.SplineMeshComponent)))